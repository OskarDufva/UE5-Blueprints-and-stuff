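; BP_BasicRotatingDoor is a door actor that swings through a quarter turn when activated.
; Its DoorInteraction event takes a timeline alpha and lerps the relative rotation of DoorPivot from zero to a fixed 90-degree offset.
; The graph contains no timeline or trigger of its own, so the caller supplies the interpolation value.
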(event EventBeginPlay
  (|CallParentFunction) ; This node is disabled and will not be called.\nDrag off pins to build functionality.
)

(event Collision|EventActorBeginOverlap
  (params (OtherActor :type Actor%20Object%20Reference))
  (|CallParentFunction OtherActor) ; This node is disabled and will not be called.\nDrag off pins to build functionality.
)

(event EventTick
  (params (DeltaSeconds :type Float%20%28single-precision%29))
  (|CallParentFunction DeltaSeconds) ; This node is disabled and will not be called.\nDrag off pins to build functionality.
)

(event EventDoorInteraction
  (params (Timeline%20alpha%20%28interpolation%29 :type Float%20%28double-precision%29))
  ;[1 1 1] Door Interaction when activated
  (Transformation|SetRelativeRotation (Variables|Default|GetDoorPivot) (Math|Rotator|Lerp(Rotator) "0, 0, 0" "0.000000,-90.000000,0.000000" Timeline%20alpha%20%28interpolation%29) false false))

(fn ConstructionScript
  (|CallParentFunction))