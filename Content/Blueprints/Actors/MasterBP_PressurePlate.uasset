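; MasterBP_PressurePlate is a pressure plate actor that pairs a plate mesh with a door child actor, likely as a base Blueprint.
; The construction script applies configurable door location, scale and rotation, plus plate location, to the components.
; BeginPlay caches the plate's original and target world locations, currently identical because the offset is zero.
; It contains no press or door-opening logic, and the node assigning the door class is unconnected.
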(event EventBeginPlay
  (bind _pressure_plate_mesh (Variables|Default|GetPressure%20Plate%20Mesh))
  (bind _returnvalue (Transformation|GetWorldLocation _pressure_plate_mesh))
  (Variables|Default|SetOriginal%20Plate%20Location _returnvalue)
  (Variables|Default|SetTarget%20Plate%20Location (- _returnvalue "")))

(fn ConstructionScript
  (bind _masterbp_doorbase (Variables|Default|GetMasterBP_DoorBase))
  ;[1 1 1] Setting locations
  (Transformation|SetRelativeLocation (Variables|Default|GetMasterBP_DoorBase) (Variables|SetLocations|GetDoor%20Location) false false)
  (Transformation|SetRelativeLocation (Variables|Default|GetPressure%20Plate%20Mesh) (Variables|SetLocations|GetPlate%20Location) false false)
  (Transformation|SetRelativeScale3D _masterbp_doorbase (Math|Conversions|ToVector(Float) (Variables|SetLocations|GetDoor%20Scale)))
  (Transformation|SetRelativeRotation _masterbp_doorbase (Variables|SetLocations|GetDoor%20Rotation) false false))