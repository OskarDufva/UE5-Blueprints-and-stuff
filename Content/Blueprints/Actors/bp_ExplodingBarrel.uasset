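; Exploding barrel actor that triggers a radial physics blast when its cylinder is hit by a first-person projectile.
; Explode draws a debug sphere at the impact point, gathers overlapping actors there and applies a velocity-change impulse from the barrel's location to those with physics-simulating roots.
; It also launches the hit actor away only if that is the first-person character, which the projectile-only trigger makes unlikely.
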(event OnComponentHit(Cylinder)
  (params (HitComponent :type Primitive%20Component%20Object%20Reference) (OtherActor :type Actor%20Object%20Reference) (OtherComp :type Primitive%20Component%20Object%20Reference) (NormalImpulse :type Vector :default "0, 0, 0") (Hit :type Hit%20Result%20Structure%20%28by%20ref%29))
  (Utilities|Casting|CastToBP_FirstPersonProjectile OtherActor)
  (CallFunction|Explode Hit))

(event EventBeginPlay)

(event Collision|EventActorBeginOverlap
  (params (OtherActor :type Actor%20Object%20Reference)))

(event EventTick
  (params (DeltaSeconds :type Float%20%28single-precision%29)))

(fn ConstructionScript)

(fn Explode
  (params (Hit :type Hit%20Result%20Structure%20%28by%20ref%29))
  (bind (_bblockinghit _binitialoverlap _time _distance _location _impactpoint _normal _impactnormal _physmat _hitactor) (Collision|BreakHitResult Hit))
  (Utilities|FlowControl|Sequence
    (:then_0
      (LocalVariables|SetImpactPoint _impactpoint)
      (Rendering|Debug|DrawDebugSphere (LocalVariables|GetImpactPoint) (Variables|Default|GetRadius) 12 "(R=1.000000,G=0.000000,B=0.000000,A=1.000000)" 5.0 2.0)
      (bind _outactors (Collision|SphereOverlapActors (LocalVariables|GetImpactPoint) (Variables|Default|GetRadius) (Utilities|Array|MakeArray "ObjectTypeQuery3" "ObjectTypeQuery4" "ObjectTypeQuery2") 0))
      (for _array_element _outactors
        (if (Physics|IsSimulatingPhysics (Variables|/Script/Engine.Actor|GetRootComponent _array_element) "None")
          (bind _asprimitive_component (Utilities|Casting|CastToPrimitiveComponent (Variables|/Script/Engine.Actor|GetRootComponent _array_element)))
          (Physics|AddRadialImpulse _asprimitive_component (Transformation|GetActorLocation) (Variables|Default|GetRadius) (Variables|Default|GetStrength) "RIF_Constant" true))))
    (:then_1
      (bind _asbp_first_person_character (Utilities|Casting|CastToBP_FirstPersonCharacter _hitactor))
      (Character|LaunchCharacter _asbp_first_person_character (* (Math|Vector|GetUnitDirection(Vector) (Transformation|GetActorLocation) (Transformation|GetActorLocation _hitactor)) (Variables|Default|GetStrength)) false false))))